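; Spline-based barbed wire Blueprint that builds a run of wire along an editable spline in the Construction Script.
; Each pair of neighboring spline points gets a spline mesh component fitted to their locations and tangents, using configurable mesh, forward axis and shadow casting.
; Two static mesh caps are then added, positioned and rotated along the spline tangent, one at the first point and one using the loop's final index for the far end.
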(fn `UserConstructionScript`
  (bind _spline1 (`self.Spline1`))
  (bind (_location _tangent) (`SplineComponent.GetLocationAndTangentAtSplinePoint` _spline1 0 "Local"))
  ;[1 1 1] points
  (for _index (range (+ (- (`SplineComponent.GetNumberOfSplinePoints` _spline1) 2) 1))
    (bind _returnvalue (`AddComponent|NODE_AddSplineMeshComponent-0`))
    ;[1 1 1] Mesh
    (`StaticMeshComponent.SetStaticMesh` _returnvalue (`self.Mesh`))
    (`SplineMeshComponent.SetForwardAxis` _returnvalue (`self.Axis`) true)
    ;[1 1 1] add point
    (`SceneComponent.K2_AttachTo` _returnvalue _spline1 "None" "KeepRelativeOffset" true)
    (bind (_location_2 _tangent_2) (`SplineComponent.GetLocationAndTangentAtSplinePoint` _spline1 _index "Local"))
    (bind (_location_3 _tangent_3) (`SplineComponent.GetLocationAndTangentAtSplinePoint` _spline1 (+ _index 1) "Local"))
    (`SplineMeshComponent.SetStartAndEnd` _returnvalue _location_2 _tangent_2 _location_3 _tangent_3 true)
    ;[1 1 1] Shadow
    (`PrimitiveComponent.SetCastShadow` _returnvalue (`self.Cast shadow`)))
  ;[1 1 1] Set cap mesh
  (bind _returnvalue_2 (`AddComponent|NODE_AddStaticMeshComponent-1`))
  ;[1 1 1] Rotate system
  (`SceneComponent.K2_SetRelativeLocation` _returnvalue_2 _location false false)
  (`SceneComponent.K2_SetRelativeRotation` _returnvalue_2 (`KismetMathLibrary.Conv_VectorToRotator` _tangent) false false)
  (bind _returnvalue_3 (`AddComponent|NODE_AddStaticMeshComponent-0`))
  (`SceneComponent.K2_SetRelativeLocation` _returnvalue_3 _location_2 false false)
  (`SceneComponent.K2_SetRelativeRotation` _returnvalue_3 (`KismetMathLibrary.Conv_VectorToRotator` _tangent_2) false false))